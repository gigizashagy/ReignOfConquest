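; Base character Blueprint combining keyboard movement with click-to-move, switching behavior on a HoldLook state that also hides the mouse cursor.
; While HoldLook is active, IA_Move strafes relative to control yaw; otherwise it moves forward/back and turns the controller with X input.
; IA_Interact traces from the cursor and paths to the hit via SimpleMoveToLocation, drawing a debug cone at the path's end on release.
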(event Input|EnhancedActionEvents|EnhancedInputActionIA_Move
  (params (ActionValue :type Vector%202D%20Structure) (ElapsedSeconds :type Float%20%28double-precision%29) (TriggeredSeconds :type Float%20%28double-precision%29) (InputAction :type Input%20Action%20Object%20Reference :default "/Game/Input/Actions/IA_Move.IA_Move"))
  (bind (_x _y) (Math|Vector2D|BreakVector2D ActionValue))
  (bind _returnvalue (Pawn|GetController))
  (bind (_x_2 _y_2) (Math|Vector2D|BreakVector2D ActionValue))
  (bind _returnvalue_2 (Pawn|GetController))
  (bind _returnvalue_3 (Pawn|GetControlRotation _returnvalue :!class /Script/Engine.Controller))
  (bind _returnvalue_4 (Pawn|GetControlRotation _returnvalue_2 :!class /Script/Engine.Controller))
  (bind _yaw (Math|Rotator|BreakRotator _returnvalue_3))
  (bind (_roll _pitch _yaw_2) (Math|Rotator|BreakRotator _returnvalue_4))
  (bind _returnvalue_5 (Math|Rotator|MakeRotator 0.0 0.0 _yaw))
  (:Triggered
    (Class|NavMovementComponent|StopActiveMovement (Variables|Character|GetCharacterMovement))
    (if (Variables|Default|GetbHoldLook)
      (Pawn|Input|AddMovementInput (Math|Vector|GetForwardVector _returnvalue_5) _y_2 false)
      (Pawn|Input|AddMovementInput (Math|Vector|GetRightVector _returnvalue_5) _x_2 false)
      (Variables|/Script/Engine.CharacterMovementComponent|SetbOrientRotationToMovement (Variables|Character|GetCharacterMovement) false)
      (else
        (Pawn|Input|AddMovementInput (Math|Vector|GetForwardVector (Math|Rotator|MakeRotator 0.0 0.0 (.Yaw (Math|Rotator|BreakRotator (Pawn|GetControlRotation (Pawn|GetController) :!class /Script/Engine.Controller))))) _y false)
        (Pawn|SetControlRotation _returnvalue_2 (Math|Rotator|MakeRotator _roll _pitch (+ _yaw_2 _x)))
        (Variables|Default|SetbUseControllerRotationYaw true)
        (Variables|/Script/Engine.CharacterMovementComponent|SetbOrientRotationToMovement (Variables|Character|GetCharacterMovement) true))))
  (:Completed
    (Variables|/Script/Engine.CharacterMovementComponent|SetbOrientRotationToMovement (Variables|Character|GetCharacterMovement) true)))

(event Input|EnhancedActionEvents|EnhancedInputActionIA_Interact
  (params (ActionValue :type Boolean) (ElapsedSeconds :type Float%20%28double-precision%29) (TriggeredSeconds :type Float%20%28double-precision%29) (InputAction :type Input%20Action%20Object%20Reference :default "/Game/Input/Actions/IA_Interact.IA_Interact"))
  (bind _returnvalue (Class|CharacterBase|GetPlayerController))
  (bind _returnvalue_2 (Class|CharacterBase|GetPlayerController))
  (bind (_worldlocation _worlddirection) (Game|Player|ConvertMouseLocationToWorldSpace _returnvalue_2))
  (bind _returnvalue_3 (Class|AIBlueprintHelperLibrary|GetCurrentPathPoints _returnvalue))
  (:Triggered
    (bind (_outhit _returnvalue_4) (Collision|LineTraceByChannel _worldlocation (+ _worldlocation (* _worlddirection 1e+04)) "TraceTypeQuery2" false 0 "None"))
    (if _returnvalue_4
      (AI|Navigation|SimpleMovetoLocation (Class|CharacterBase|GetPlayerController) (.Location (Collision|BreakHitResult _outhit)))
      (Variables|/Script/Engine.CharacterMovementComponent|SetbOrientRotationToMovement (Variables|Character|GetCharacterMovement) true)
      (Variables|Default|SetbUseControllerRotationYaw false)))
  (:Completed
    (if (Utilities|Array|IsNotEmpty _returnvalue_3)
      (Class|KismetSystemLibrary|DrawDebugConeinDegrees (Utilities|Array|Get(acopy) _returnvalue_3 (Utilities|Array|LastIndex _returnvalue_3)) "0.000000,0.000000,1.000000" 5e+01 45.0 45.0 4 "(R=0.012786,G=0.000000,B=1.000000,A=1.000000)" 5.0 0.0))))

(event EventHoldLook
  (params (Value :type Input%20Action%20Value%20Structure%20%28by%20ref%29))
  (|CallParentFunction Value)
  (Variables|/Script/Engine.PlayerController|SetbShowMouseCursor (Class|CharacterBase|GetPlayerController) (not (Variables|Default|GetbHoldLook)))
  (Variables|Default|SetbUseControllerRotationYaw false))

(fn ConstructionScript)